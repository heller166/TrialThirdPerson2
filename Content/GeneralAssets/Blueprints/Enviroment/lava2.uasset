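; Lava hazard actor that hurts the player character on contact.
; When MyCharacter_InUse enters the Box, it makes the character jump, spawns an explosion particle at its location, subtracts FireDamage from its clamped HealthValue and plays the Explosion component.
; A DoOnce gate limits this to one hit until the character leaves the box, which resets it.
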(event OnComponentEndOverlap(Box)
  (params (OtherActor :type Actor%20Object%20Reference) (OtherComp :type Primitive%20Component%20Object%20Reference) (OtherBodyIndex :type Integer))
  (Utilities|Casting|CastToMyCharacter_InUse OtherActor)
  (Utilities|FlowControl|DoOnce false) ; enters at Reset
)

(event OnComponentBeginOverlap(Box)
  (params (OtherActor :type Actor%20Object%20Reference) (OtherComp :type Primitive%20Component%20Object%20Reference) (OtherBodyIndex :type Integer) (bFromSweep :type Boolean) (SweepResult :type Hit%20Result%20Structure%20%28by%20ref%29))
  (Utilities|FlowControl|DoOnce false
    (:Completed
      (bind _asmy_character_in_use (Utilities|Casting|CastToMyCharacter_InUse OtherActor))
      (bind _output_get (Variables|Default|SetCharacterReference _asmy_character_in_use))
      (Character|Jump _output_get)
      (Effects|SpawnEmitteratLocation "/Game/GeneralAssets/Particles/P_Explosion.P_Explosion" (Transformation|GetActorLocation _output_get))
      (Variables|/Game/ThirdPersonBP/MyCharacter_InUse.MyCharacter_InUse_C|SetHealthValue _output_get (Math|Float|Clamp(Float) (- (Variables|/Game/ThirdPersonBP/MyCharacter_InUse.MyCharacter_InUse_C|GetHealthValue _output_get) (Variables|Default|GetFireDamage)) -0.1))
      (Audio|Components|Audio|Play (Variables|Default|GetExplosion) 0.0))))

(fn ConstructionScript)