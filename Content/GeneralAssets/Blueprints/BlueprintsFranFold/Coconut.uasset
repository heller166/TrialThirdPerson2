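; Coconut is a pickup item that the player stores in the inventory and later uses to change health, energy and heart rate.
; A trigger overlap toggles a prompt widget and an in-range flag that gates pickup through an event bound on the character.
; Pickup adds the item struct to the HUD inventory and hides the actor.
; UseAction applies clamped stat changes, then destroys it.
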(event OnComponentBeginOverlap(Trigger)
  (params (OtherActor :type Actor%20Object%20Reference) (OtherComp :type Primitive%20Component%20Object%20Reference) (OtherBodyIndex :type Integer) (bFromSweep :type Boolean) (SweepResult :type Hit%20Result%20Structure%20%28by%20ref%29))
  (bind _pickuptextcoconutreference (Variables|Default|GetPickUpTextCoconutReference))
  ;[1 1 1] PickUpText Trigger
  (Utilities|Casting|CastToMyCharacter_InUse OtherActor)
  (UserInterface|Viewport|AddtoViewport _pickuptextcoconutreference 0)
  (Widget|SetVisibility _pickuptextcoconutreference "Visible")
  (Variables|Default|SetIsinRange? true))

(event OnComponentEndOverlap(Trigger)
  (params (OtherActor :type Actor%20Object%20Reference) (OtherComp :type Primitive%20Component%20Object%20Reference) (OtherBodyIndex :type Integer))
  ;[1 1 1] PickUpText Trigger
  (Utilities|Casting|CastToMyCharacter_InUse OtherActor)
  (Widget|SetVisibility (Variables|Default|GetPickUpTextCoconutReference) "Hidden")
  (Variables|Default|SetIsinRange? false))

(event Custom|PickUpItem_Event_1
  (bind _characterreference (Variables|Default|GetCharacterReference))
  (bind _gamehudreference (Variables|/Game/ThirdPersonBP/MyCharacter_InUse.MyCharacter_InUse_C|GetGameHUDReference _characterreference))
  ;[1 1 1] PickUp and add items to inventory and refresh it
  (if (and (Collision|GetActorEnableCollision) (Variables|Default|GetIsinRange?))
    (Utilities|Array|Add (Variables|/Game/GeneralAssets/UMG/surviveHUD.surviveHUD_C|GetInventoryReference _gamehudreference) (Variables|Default|GetItemInfo))
    (Widget|RemovefromParent (Variables|Default|GetPickUpTextCoconutReference))
    (Rendering|SetActorHiddenInGame true)
    (Collision|SetActorEnableCollision false)
    (Default|RefreshInventory _gamehudreference)))

(event EventBeginPlay
  (bind _iteminfo (Variables|Default|GetItemInfo))
  (bind (_item _itemimage _pickuptext) (Utilities|Struct|BreakInventory_Struct _iteminfo))
  ;[1 1 1] Event Begin Play
  (bind _returnvalue (UserInterface|CreateWidget "/Game/GeneralAssets/UMG/PickupTextCoconut.PickupTextCoconut_C"))
  (Variables|Default|SetPickUpTextCoconutReference _returnvalue)
  (Utilities|Struct|SetmembersinInventory_Struct _iteminfo self)
  (Variables|/Game/GeneralAssets/UMG/PickupTextCoconut.PickupTextCoconut_C|SetPickUpActor (Variables|Default|GetPickUpTextCoconutReference) _item)
  (Variables|/Game/GeneralAssets/UMG/PickupTextCoconut.PickupTextCoconut_C|SetPickUpText (Variables|Default|GetPickUpTextCoconutReference) _pickuptext)
  (bind _asmy_character_in_use (Utilities|Casting|CastToMyCharacter_InUse (Game|GetPlayerCharacter 0)))
  (bind _output_get (Variables|Default|SetCharacterReference _asmy_character_in_use))
  (EventDispatchers|AssignPickUpItem _output_get (delegate Custom|PickUpItem_Event_1))
  (Utilities|FlowControl|Delay 1.0)
  (Physics|SetSimulatePhysics (Variables|Default|GetStaticMesh) false))

(event EventUseAction
  (bind _characterreference (Variables|Default|GetCharacterReference))
  ;[1 1 1] Item Use Fuctionality
  (Variables|/Game/ThirdPersonBP/MyCharacter_InUse.MyCharacter_InUse_C|SetHealthValue _characterreference (Math|Float|Clamp(Float) (+ (Variables|/Game/ThirdPersonBP/MyCharacter_InUse.MyCharacter_InUse_C|GetHealthValue _characterreference) (Variables|Default|GetaddHealth))))
  (Variables|/Game/ThirdPersonBP/MyCharacter_InUse.MyCharacter_InUse_C|SetEnergyValue _characterreference (Math|Float|Clamp(Float) (+ (Variables|/Game/ThirdPersonBP/MyCharacter_InUse.MyCharacter_InUse_C|GetEnergyValue _characterreference) (Variables|Default|GetaddEnergy))))
  (Variables|/Game/ThirdPersonBP/MyCharacter_InUse.MyCharacter_InUse_C|SetHeartRateValue _characterreference (Math|Float|Clamp(Float) (+ (Variables|/Game/ThirdPersonBP/MyCharacter_InUse.MyCharacter_InUse_C|GetHeartRateValue _characterreference) (Variables|Default|GetaddHeartRate))))
  (Actor|DestroyActor))

(fn ConstructionScript
  (Utilities|Struct|SetmembersinInventory_Struct (Variables|Default|GetItemInfo) self (Variables|Default|GetCustomImage) (Variables|Default|GetCustomPickupText) (Variables|Default|GetCustomActionText))
  (Components|StaticMesh|SetStaticMesh (Variables|Default|GetStaticMesh) (Variables|Default|GetCustomStaticMesh)))