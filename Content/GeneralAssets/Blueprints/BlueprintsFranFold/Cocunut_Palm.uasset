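; Coconut palm actor that drops a single pickup-style CrabMeat actor after taking enough damage.
; While HasCoconut is set, AnyDamage subtracts floored damage from Health, then clears the flag and calls CoconutSpawn once Health is depleted.
; CoconutSpawn creates CrabMeat below the palm's origin with its rotation and scale; debug prints trace the flow.
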(event Custom|CoconutSpawn
  (bind _returnvalue (Transformation|GetActorTransform))
  (bind (_location _rotation _scale) (Math|Transform|BreakTransform _returnvalue))
  ;[1 1 1] CoconutSpawn
  (Development|PrintString "Hello2")
  (Game|SpawnActorfromClass "/Game/GeneralAssets/Blueprints/BlueprintsFranFold/CrabMeat.CrabMeat_C" (Math|Transform|MakeTransform (+ _location "0, 0,-90.000000") _rotation _scale) "Undefined" 0 0)
  (Development|PrintString "after"))

(event EventBeginPlay)

(event Game|Damage|EventAnyDamage
  (params (Damage :type Float%20%28single-precision%29) (DamageType :type Damage%20Type%20Object%20Reference) (InstigatedBy :type Controller%20Object%20Reference) (DamageCauser :type Actor%20Object%20Reference))
  ;[1 1 1] Damage
  (Development|PrintString "Hello")
  (if (Variables|Default|GetHasCoconut)
    (Variables|Default|SetHealth (- (Variables|Default|GetHealth) (Math|Float|Floor Damage)))
    (Development|PrintString "Hello3")
    (if (<= (Variables|Default|GetHealth) 0)
      (Variables|Default|SetHasCoconut false)
      (CallFunction|CoconutSpawn))))

(fn ConstructionScript)