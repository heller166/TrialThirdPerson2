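; CrabPointsBP is a crab enemy character that jump-attacks the player and drops crab meat when killed.
; Sight overlap caches the player reference, while MeleeRange overlap starts and stops a looping JumpAttack timer that hops and subtracts directly from the player's HealthValue.
; AnyDamage lowers Health by the floored damage; at zero the mesh simulates physics, spawns CrabMeat after a short delay, then destroys the actor.
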(event OnComponentEndOverlap(MeleeRange)
  (params (OtherActor :type Actor%20Object%20Reference) (OtherComp :type Primitive%20Component%20Object%20Reference) (OtherBodyIndex :type Integer))
  ;[1 1 1] AttackOn/Off
  (Utilities|Casting|CastToMyCharacter_InUse OtherActor)
  (Class|KismetSystemLibrary|ClearTimerHandle (stale OnComponentBeginOverlap(MeleeRange) _returnvalue)))

(event OnComponentBeginOverlap(Sight)
  (params (OtherActor :type Actor%20Object%20Reference) (OtherComp :type Primitive%20Component%20Object%20Reference) (OtherBodyIndex :type Integer) (bFromSweep :type Boolean) (SweepResult :type Hit%20Result%20Structure%20%28by%20ref%29))
  ;[1 1 1] CastWhenInSight
  (bind _asmy_character_in_use (Utilities|Casting|CastToMyCharacter_InUse OtherActor))
  (Variables|Default|SetCharacterReference _asmy_character_in_use))

(event OnComponentBeginOverlap(MeleeRange)
  (params (OtherActor :type Actor%20Object%20Reference) (OtherComp :type Primitive%20Component%20Object%20Reference) (OtherBodyIndex :type Integer) (bFromSweep :type Boolean) (SweepResult :type Hit%20Result%20Structure%20%28by%20ref%29))
  ;[1 1 1] AttackOn/Off
  (Utilities|Casting|CastToMyCharacter_InUse OtherActor)
  (bind _returnvalue (Utilities|Time|SetTimerbyFunctionName 0 "JumpAttack" 0.6 true)))

(event Custom|Death
  ;[1 1 1] Death
  (Physics|SetSimulatePhysics (Variables|Character|GetMesh) true)
  (Utilities|FlowControl|Delay 0.7)
  (Game|SpawnActorfromClass "/Game/GeneralAssets/Blueprints/BlueprintsFranFold/CrabMeat.CrabMeat_C" (Math|Transform|MakeTransform (Math|Transform|TransformLocation (Transformation|GetActorTransform) "0, 0,-85.000000")) "Undefined" 0 0)
  (Utilities|FlowControl|Delay 3.0)
  (Actor|DestroyActor))

(event Game|Damage|EventAnyDamage
  (params (Damage :type Float%20%28single-precision%29) (DamageType :type Damage%20Type%20Object%20Reference) (InstigatedBy :type Controller%20Object%20Reference) (DamageCauser :type Actor%20Object%20Reference))
  ;[1 1 1] Damage
  (if (Variables|Default|GetAlive)
    (Variables|Default|SetHealth (- (Variables|Default|GetHealth) (Math|Float|Floor Damage)))
    (if (<= (Variables|Default|GetHealth) 0)
      (Variables|Default|SetAlive false)
      (CallFunction|Death))))

(fn ConstructionScript)

(fn JumpAttack
  (bind _characterreference (Variables|Default|GetCharacterReference))
  (if (Variables|Default|GetAlive)
    (Character|Jump)
    (Variables|/Game/ThirdPersonBP/MyCharacter_InUse.MyCharacter_InUse_C|SetHealthValue _characterreference (- (Variables|/Game/ThirdPersonBP/MyCharacter_InUse.MyCharacter_InUse_C|GetHealthValue _characterreference) (Variables|Default|GetDamage)))))