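; Tutorial crab enemy that speeds up on sighting the player, jump-attacks in melee range and drops crab meat on death.
; Sight overlap caches the player reference; melee overlap runs a looping timer that jumps and applies damage.
; Taking damage reduces health and starts a brief gated Delay loop that interpolates the crab toward the player's PushLocation as knockback.
; Death enables mesh physics, spawns meat at a downward-trace hit, then destroys the actor.
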(event OnComponentEndOverlap(MeleeRange)
  (params (OtherActor :type Actor%20Object%20Reference) (OtherComp :type Primitive%20Component%20Object%20Reference) (OtherBodyIndex :type Integer))
  ;[1 1 1] AttackOn/Off
  (Utilities|Casting|CastToMyCharacter_InUse OtherActor)
  (Class|KismetSystemLibrary|ClearTimerHandle (stale OnComponentBeginOverlap(MeleeRange) _returnvalue)))

(event OnComponentBeginOverlap(Sight)
  (params (OtherActor :type Actor%20Object%20Reference) (OtherComp :type Primitive%20Component%20Object%20Reference) (OtherBodyIndex :type Integer) (bFromSweep :type Boolean) (SweepResult :type Hit%20Result%20Structure%20%28by%20ref%29))
  ;[1 1 1] CastWhenInSight
  (bind _asmy_character_in_use (Utilities|Casting|CastToMyCharacter_InUse OtherActor))
  (Variables|Default|SetCharacterReference _asmy_character_in_use)
  (Variables|/Script/Engine.CharacterMovementComponent|SetMaxWalkSpeed (Variables|Character|GetCharacterMovement) 6e+02))

(event OnComponentBeginOverlap(MeleeRange)
  (params (OtherActor :type Actor%20Object%20Reference) (OtherComp :type Primitive%20Component%20Object%20Reference) (OtherBodyIndex :type Integer) (bFromSweep :type Boolean) (SweepResult :type Hit%20Result%20Structure%20%28by%20ref%29))
  ;[1 1 1] AttackOn/Off
  (Utilities|Casting|CastToMyCharacter_InUse OtherActor)
  (bind _returnvalue (Utilities|Time|SetTimerbyFunctionName 0 "JumpAttack" 0.6 true)))

(event Custom|Push
  ;[1 1 1] Push
  (Transformation|SetActorLocation (Math|Interpolation|VInterpTo (Transformation|GetActorLocation) (.Location (Math|Transform|BreakTransform (Transformation|GetWorldTransform (Variables|/Game/ThirdPersonBP/MyCharacter_InUse.MyCharacter_InUse_C|GetPushLocation (Variables|Default|GetCharacterReference))))) (Utilities|Time|GetWorldDeltaSeconds) 2.0) false false :!label _label)
  (Utilities|FlowControl|Delay 0.01)
  (Utilities|FlowControl|Sequence
    (:then_0
      (Utilities|FlowControl|Gate true :!label _label_2
        (:Exit
          (goto _label))))
    (:then_1
      (Utilities|FlowControl|Delay 1.0)
      (goto _label_2 Close))))

(event Custom|OpenDoorPush
  ;[1 1 1] Push
  (Utilities|FlowControl|Gate true) ; enters at Open
)

(event Custom|Death
  (bind _returnvalue (Transformation|GetActorLocation))
  (bind (_x _y) (Math|Vector|BreakVector _returnvalue))
  ;[1 1 1] Death
  (bind _outhit (Collision|LineTraceByChannel (Transformation|GetActorLocation) (Math|Vector|MakeVector _x _y -1e+03) "TraceTypeQuery1" false 0 "None"))
  (Physics|SetSimulatePhysics (Variables|Character|GetMesh) true)
  (Utilities|FlowControl|Delay 0.7)
  (Game|SpawnActorfromClass "/Game/GeneralAssets/Blueprints/BlueprintsFranFold/CrabMeat.CrabMeat_C" (Math|Transform|MakeTransform (.Location (Collision|BreakHitResult _outhit))) "Undefined" 0 0)
  (Utilities|FlowControl|Delay 3.0)
  (Actor|DestroyActor))

(event EventBeginPlay
  ;[1 1 1] SetRestSpeed
  (Variables|/Script/Engine.CharacterMovementComponent|SetMaxWalkSpeed (Variables|Character|GetCharacterMovement) 2e+02))

(event Game|Damage|EventAnyDamage
  (params (Damage :type Float%20%28single-precision%29) (DamageType :type Damage%20Type%20Object%20Reference) (InstigatedBy :type Controller%20Object%20Reference) (DamageCauser :type Actor%20Object%20Reference))
  ;[1 1 1] Damage
  (CallFunction|Push)
  (CallFunction|OpenDoorPush)
  (if (Variables|Default|GetAlive)
    (Variables|Default|SetHealth (- (Variables|Default|GetHealth) (Math|Float|Floor Damage)))
    (if (<= (Variables|Default|GetHealth) 0)
      (Variables|Default|SetAlive false)
      (CallFunction|Death))))

(fn ConstructionScript)

(fn JumpAttack
  (if (Variables|Default|GetAlive)
    (Character|Jump)
    (Game|Damage|ApplyDamage (Variables|Default|GetCharacterReference) (Variables|Default|GetDamage) 0 self)
    (Development|PrintString "damage")))