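; Crab enemy that tracks the player through Sight and MeleeRange overlaps, takes damage, and drops CrabMeat on death.
; Melee timers repeat DoubleJump repositioning and a JumpAttack that only traces, with its damage call unwired.
; Double jumps, push-back on damage and Tick-driven catch-up use gated Delay loops interpolating the crab toward points on the player.
; Death enables mesh physics, spawns meat at a downward trace hit and destroys the actor.
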(event OnComponentEndOverlap(Sight)
  (params (OtherActor :type Actor%20Object%20Reference) (OtherComp :type Primitive%20Component%20Object%20Reference) (OtherBodyIndex :type Integer))
  ;[1 1 1] CastWhenInSight & CheckIfInRange
  (Utilities|Casting|CastToMyCharacter_InUse OtherActor)
  (Variables|Default|SetIsInRange? false))

(event OnComponentEndOverlap(MeleeRange)
  (params (OtherActor :type Actor%20Object%20Reference) (OtherComp :type Primitive%20Component%20Object%20Reference) (OtherBodyIndex :type Integer))
  ;[1 1 1] AttackOn/Off
  (Utilities|Casting|CastToMyCharacter_InUse OtherActor)
  (Class|KismetSystemLibrary|ClearTimerHandle (stale OnComponentBeginOverlap(MeleeRange) _returnvalue))
  (Class|KismetSystemLibrary|ClearTimerHandle (stale OnComponentBeginOverlap(MeleeRange) _returnvalue_2)))

(event OnComponentBeginOverlap(Sight)
  (params (OtherActor :type Actor%20Object%20Reference) (OtherComp :type Primitive%20Component%20Object%20Reference) (OtherBodyIndex :type Integer) (bFromSweep :type Boolean) (SweepResult :type Hit%20Result%20Structure%20%28by%20ref%29))
  ;[1 1 1] CastWhenInSight & CheckIfInRange
  (bind _asmy_character_in_use (Utilities|Casting|CastToMyCharacter_InUse OtherActor))
  (Variables|Default|SetCharacterReference _asmy_character_in_use)
  (Variables|/Script/Engine.CharacterMovementComponent|SetMaxWalkSpeed (Variables|Character|GetCharacterMovement) 6e+02)
  (Variables|Default|SetIsInRange? true))

(event OnComponentBeginOverlap(MeleeRange)
  (params (OtherActor :type Actor%20Object%20Reference) (OtherComp :type Primitive%20Component%20Object%20Reference) (OtherBodyIndex :type Integer) (bFromSweep :type Boolean) (SweepResult :type Hit%20Result%20Structure%20%28by%20ref%29))
  ;[1 1 1] AttackOn/Off
  (Utilities|Casting|CastToMyCharacter_InUse OtherActor)
  (bind _returnvalue (Utilities|Time|SetTimerbyFunctionName 0 "JumpAttack" 0.6 true))
  (bind _returnvalue_2 (Utilities|Time|SetTimerbyFunctionName 0 "DoubleJump" 3.0 true)))

(event OnComponentBeginOverlap(NoNeedCatchUpRange)
  (params (OtherActor :type Actor%20Object%20Reference) (OtherComp :type Primitive%20Component%20Object%20Reference) (OtherBodyIndex :type Integer) (bFromSweep :type Boolean) (SweepResult :type Hit%20Result%20Structure%20%28by%20ref%29))
  ;[1 1 1] CatchUpRange
)

(event OnComponentEndOverlap(NoNeedCatchUpRange)
  (params (OtherActor :type Actor%20Object%20Reference) (OtherComp :type Primitive%20Component%20Object%20Reference) (OtherBodyIndex :type Integer))
  ;[1 1 1] CatchUpRange
)

(event Custom|Push
  ;[1 1 1] Push
  (Transformation|SetActorLocation (Math|Interpolation|VInterpTo (Transformation|GetActorLocation) (.Location (Math|Transform|BreakTransform (Transformation|GetWorldTransform (Variables|/Game/ThirdPersonBP/MyCharacter_InUse.MyCharacter_InUse_C|GetPushLocation (Variables|Default|GetCharacterReference))))) (Utilities|Time|GetWorldDeltaSeconds) 2.0) false false :!label _label)
  (Utilities|FlowControl|Delay 0.01)
  (Utilities|FlowControl|Sequence
    (:then_0
      (Utilities|FlowControl|Gate true :!label _label_2
        (:Exit
          (goto _label))))
    (:then_1
      (Utilities|FlowControl|Delay 1.0)
      (goto _label_2 Close))))

(event Custom|CatchUp
  (bind _characterreference (Variables|Default|GetCharacterReference))
  ;[1 1 1] CatchUp
  (Utilities|FlowControl|DoOnce false
    (:Completed
      (Development|PrintString "catch")
      (Variables|Default|SetNewTergetCatchUp (Utilities|Array|Get(acopy) (Utilities|Array|MakeArray (Transformation|GetWorldLocation (Variables|/Game/ThirdPersonBP/MyCharacter_InUse.MyCharacter_InUse_C|GetCatchUp0 _characterreference)) (Transformation|GetWorldLocation (Variables|/Game/ThirdPersonBP/MyCharacter_InUse.MyCharacter_InUse_C|GetCatchUp1 _characterreference)) (Transformation|GetWorldLocation (Variables|/Game/ThirdPersonBP/MyCharacter_InUse.MyCharacter_InUse_C|GetCatchUp2 _characterreference))) (Math|Random|RandomInteger 3)))
      (Transformation|SetActorLocation (Math|Interpolation|VInterpTo (Transformation|GetActorLocation) (Variables|Default|GetNewTergetCatchUp) (Utilities|Time|GetWorldDeltaSeconds) 4.0) false false :!label _label)
      (Utilities|FlowControl|Delay 0.01)
      (Utilities|FlowControl|Sequence
        (:then_0
          (Utilities|FlowControl|Gate true :!label _label_2
            (:Exit
              (goto _label))))
        (:then_1
          (Utilities|FlowControl|Delay 0.6)
          (goto _label_2 Close))))))

(event Custom|OpenDoorMoveOnLoc
  ;[1 1 1] DoubleJump
  (Utilities|FlowControl|Gate true) ; enters at Open
)

(event Custom|OpenDoorMoveOnRot
  (Utilities|FlowControl|Gate true) ; enters at Open
)

(event Custom|MoveOnTopLoc
  (bind _characterreference (Variables|Default|GetCharacterReference))
  ;[1 1 1] DoubleJump
  (Variables|Default|SetNewTargetDoubleJump (Utilities|Array|Get(acopy) (Utilities|Array|MakeArray (Transformation|GetWorldLocation (Variables|/Game/ThirdPersonBP/MyCharacter_InUse.MyCharacter_InUse_C|GetDoubleJumpLocation0 _characterreference)) (Transformation|GetWorldLocation (Variables|/Game/ThirdPersonBP/MyCharacter_InUse.MyCharacter_InUse_C|GetDoubleJumpLocation1 _characterreference)) (Transformation|GetWorldLocation (Variables|/Game/ThirdPersonBP/MyCharacter_InUse.MyCharacter_InUse_C|GetDoubleJumpLocation2 _characterreference)) (Transformation|GetWorldLocation (Variables|/Game/ThirdPersonBP/MyCharacter_InUse.MyCharacter_InUse_C|GetDoubleJumpLocation3 _characterreference))) (Math|Random|RandomInteger 4)))
  (Transformation|SetActorLocation (Math|Interpolation|VInterpTo (Transformation|GetActorLocation) (Variables|Default|GetNewTargetDoubleJump) (Utilities|Time|GetWorldDeltaSeconds) 1.0) false false :!label _label)
  (Utilities|FlowControl|Delay 0.01)
  (Utilities|FlowControl|Sequence
    (:then_0
      (Utilities|FlowControl|Gate true :!label _label_2
        (:Exit
          (goto _label))))
    (:then_1
      (Utilities|FlowControl|Delay 1.0)
      (goto _label_2 Close))))

(event Custom|OpenDoorPush
  ;[1 1 1] Push
  (Utilities|FlowControl|Gate true) ; enters at Open
)

(event Custom|OpenDoorCatchUp
  ;[1 1 1] CatchUp
  (Utilities|FlowControl|Gate true) ; enters at Open
)

(event Custom|MoveOnTopRot
  (Transformation|SetActorRotation (Math|Interpolation|RInterpTo (Transformation|GetActorRotation) (Transformation|GetActorRotation) (Utilities|Time|GetWorldDeltaSeconds) 0.0) :!label _label)
  (Utilities|FlowControl|Delay 0.01)
  (Utilities|FlowControl|Sequence
    (:then_0
      (Utilities|FlowControl|Gate true :!label _label_2
        (:Exit
          (goto _label))))
    (:then_1
      (Utilities|FlowControl|Delay 1.0)
      (goto _label_2 Close))))

(event Custom|Death
  (bind _returnvalue (Transformation|GetActorLocation))
  (bind (_x _y) (Math|Vector|BreakVector _returnvalue))
  ;[1 1 1] Death
  (bind _outhit (Collision|LineTraceByChannel (Transformation|GetActorLocation) (Math|Vector|MakeVector _x _y -1e+03) "TraceTypeQuery1" false 0 "None"))
  (Physics|SetSimulatePhysics (Variables|Character|GetMesh) true)
  (Utilities|FlowControl|Delay 0.7)
  (Game|SpawnActorfromClass "/Game/GeneralAssets/Blueprints/BlueprintsFranFold/CrabMeat.CrabMeat_C" (Math|Transform|MakeTransform (.Location (Collision|BreakHitResult _outhit))) "Undefined" 0 0)
  (Utilities|FlowControl|Delay 3.0)
  (Actor|DestroyActor))

(event EventBeginPlay
  ;[1 1 1] SetRestSpeed
  (Variables|/Script/Engine.CharacterMovementComponent|SetMaxWalkSpeed (Variables|Character|GetCharacterMovement) 2e+02))

(event EventTick
  (params (DeltaSeconds :type Float%20%28single-precision%29))
  (bind _characterreference (Variables|Default|GetCharacterReference))
  ;[1 1 1] CheckIfNeedToCatchUp
  (if (Variables|Default|GetIsInRange?)
    (for _array_element (Collision|GetOverlappingActors (Variables|Default|GetNoNeedCatchUpRange) 0 :!class /Script/Engine.PrimitiveComponent)
      (if (not (Collision|IsOverlappingActor _array_element (Variables|Default|GetCharacterReference) :!class /Script/Engine.Actor))
        (CallFunction|CatchUp)
        (CallFunction|OpenDoorCatchUp)
        (Utilities|FlowControl|Delay (Math|Conversions|ToFloat(Integer) (Math|Random|RandomIntegerinRange 2 6)))
        ;[1 1 1] CatchUp
        (Utilities|FlowControl|DoOnce false) ; enters at Reset
      ))))

(event Game|Damage|EventAnyDamage
  (params (Damage :type Float%20%28single-precision%29) (DamageType :type Damage%20Type%20Object%20Reference) (InstigatedBy :type Controller%20Object%20Reference) (DamageCauser :type Actor%20Object%20Reference))
  ;[1 1 1] Damage
  (CallFunction|Push)
  (CallFunction|OpenDoorPush)
  (if (Variables|Default|GetAlive)
    (Variables|Default|SetHealth (- (Variables|Default|GetHealth) (Math|Float|Floor Damage)))
    (if (<= (Variables|Default|GetHealth) 0)
      (Variables|Default|SetAlive false)
      (CallFunction|Death))))

(fn ConstructionScript)

(fn JumpAttack
  (if (Variables|Default|GetAlive)
    (Collision|LineTraceByChannel (Transformation|GetActorLocation) "0, 0, 0" "TraceTypeQuery1" false 0 "None")))

(fn DoubleJump
  (CallFunction|MoveonTopLoc)
  (CallFunction|OpenDoorMoveonLoc))

(fn CatchUpFunc
  (CallFunction|CatchUp)
  (CallFunction|OpenDoorCatchUp)
  (Development|PrintString "CATCH"))